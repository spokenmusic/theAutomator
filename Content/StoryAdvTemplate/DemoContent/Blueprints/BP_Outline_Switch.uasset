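; BP_Outline_Switch is a demo interactable from the story adventure template that toggles the outline effect off and on.
; Its Interaction event runs a FlipFlop that disables, then re-enables, the first PostProcessVolume found in the level and prints the new state.
; The switch looks up the volume on every use and assumes that the first one carries the outlines, starting enabled.
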(event EventInteraction
  (params (Character :type BP%20First%20Person%20Character%20Object%20Reference))
  (Utilities|FlowControl|FlipFlop
    (:A
      (bind _outactors (Actor|GetAllActorsOfClass "/Script/Engine.PostProcessVolume"))
      (Variables|/Script/Engine.PostProcessVolume|SetbEnabled (Utilities|Array|Get(acopy) _outactors) false)
      (Development|PrintString "Outlines disabled"))
    (:B
      (bind _outactors_2 (Actor|GetAllActorsOfClass "/Script/Engine.PostProcessVolume"))
      (Variables|/Script/Engine.PostProcessVolume|SetbEnabled (Utilities|Array|Get(acopy) _outactors_2) true)
      (Development|PrintString "Outlines enabled"))))

(fn ConstructionScript
  (|CallParentFunction))