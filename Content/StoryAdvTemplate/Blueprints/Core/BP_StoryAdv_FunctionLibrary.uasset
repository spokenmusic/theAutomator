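; Blueprint function library for the story adventure template with shared player-control and object-inspection helpers.
; Two functions lock and restore movement by toggling player 0 pawn input, with the lock also stopping current movement immediately.
; Two others turn X and Y input into inspection rotation deltas, using trigonometry on the camera's forward vector to keep rotation view-relative, scaled by delta time and speed.
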(fn DisablePlayerMovement
  (Input|DisableInput (Game|Player|GetPlayerPawn 0) (Game|GetPlayerController 0))
  (Components|Movement|StopMovementImmediately (Pawn|GetMovementComponent (Game|Player|GetPlayerPawn 0))))

(fn EnablePlayerMovement
  (Input|EnableInput (Game|Player|GetPlayerPawn 0) (Game|GetPlayerController 0)))

(fn CaclulateInpsectionRotationY
  (params (InputValue :type Float%20%28single-precision%29) (RotationSpeed :type Float%20%28single-precision%29))
  (LocalVariables|SetCameraForwardVector (Transformation|GetActorForwardVector (Game|GetPlayerCameraManager (LocalVariables|Get__WorldContext))))
  (return (* (* (Math|Rotator|MakeRotator (* InputValue (Math|Trig|Sin(Degrees) (.yaw (Math|Rotator|MakeRotfromX (LocalVariables|GetCameraForwardVector)))) -1.0) (* InputValue (Math|Trig|Sin(Degrees) (.yaw (Math|Rotator|MakeRotfromX (Math|Vector|RotateVectorAroundAxis (LocalVariables|GetCameraForwardVector) 9e+01 "0.000000,0.000000,1.000000"))))) 0.0) (Utilities|Time|GetWorldDeltaSeconds (LocalVariables|Get__WorldContext))) RotationSpeed)))

(fn CaclulateInpsectionRotationX
  (params (InputValue :type Float%20%28single-precision%29) (RotationSpeed :type Float%20%28single-precision%29))
  (LocalVariables|SetCameraForwardVector (Transformation|GetActorForwardVector (Game|GetPlayerCameraManager (LocalVariables|Get__WorldContext))))
  (return (* (* (Math|Rotator|MakeRotator (* InputValue (Math|Trig|Sin(Degrees) (.pitch (Math|Rotator|MakeRotfromX (LocalVariables|GetCameraForwardVector)))) (Math|Trig|Cos(Degrees) (.yaw (Math|Rotator|MakeRotfromX (LocalVariables|GetCameraForwardVector)))) -1.0) (* InputValue (Math|Trig|Sin(Degrees) (.pitch (Math|Rotator|MakeRotfromX (LocalVariables|GetCameraForwardVector)))) (Math|Trig|Sin(Degrees) (.yaw (Math|Rotator|MakeRotfromX (LocalVariables|GetCameraForwardVector)))) -1.0) (* InputValue (Math|Trig|Cos(Degrees) (.pitch (Math|Rotator|MakeRotfromX (LocalVariables|GetCameraForwardVector)))) -1.0)) (Utilities|Time|GetWorldDeltaSeconds (LocalVariables|Get__WorldContext))) RotationSpeed)))