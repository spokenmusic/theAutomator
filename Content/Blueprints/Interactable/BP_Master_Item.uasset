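; Master pickup item actor that gives its item to an interacting character.
; The Interaction event adds the ItemID and Quantity to the character's Inventory, then destroys the actor unless it is an infinite resource.
; A failed add prints a message instead.
; The construction script shows the ItemID on a text render component for identification.
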(event EventBeginPlay)

(event Collision|EventActorBeginOverlap
  (params (OtherActor :type Actor%20Object%20Reference)))

(event EventTick
  (params (DeltaSeconds :type Float%20%28single-precision%29)))

(event EventInteraction
  (params (Character :type BP%20First%20Person%20Character%20Object%20Reference))
  (bind _returnvalue (Class|InventoryComponent|AddItem (Variables|/Game/Blueprints/Core/BP_FirstPersonCharacter.BP_FirstPersonCharacter_C|GetInventory Character) (Variables|Default|GetItemID) (Variables|Default|GetQuantity)))
  (if _returnvalue
    (if (not (Variables|Default|GetInfinite%20Resource))
      (Actor|DestroyActor))
    (else
      (Development|PrintString "Can't add item"))))

(fn ConstructionScript
  (|CallParentFunction)
  (Rendering|Components|TextRender|SetText (Variables|Default|GetTextRender) (Utilities|Text|ToText(Name) (Variables|Default|GetItemID))))