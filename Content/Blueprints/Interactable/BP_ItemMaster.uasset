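; BP_ItemMaster is an item actor, filed under Interactable, that labels itself with a TextRender component.
; The construction script sets the label to the raw ItemID.
; On BeginPlay, it replaces that with the DisplayName from the item definition that ItemDataSubsystem returns for the ItemID.
; It has no active overlap or tick logic.
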(event EventBeginPlay
  (bind _returnvalue (Class|ItemDataSubsystem|GetItemDataSubsystem))
  (Rendering|Components|TextRender|SetText (Variables|Default|GetTextRender) (.DisplayName (Utilities|Struct|BreakItemData (Class|ItemDataSubsystem|GetItemDefinition _returnvalue (Variables|Default|GetItemID))))))

(event Collision|EventActorBeginOverlap
  (params (OtherActor :type Actor%20Object%20Reference)))

(event EventTick
  (params (DeltaSeconds :type Float%20%28single-precision%29)))

(fn ConstructionScript
  (Rendering|Components|TextRender|SetText (Variables|Default|GetTextRender) (Utilities|Text|ToText(Name) (Variables|Default|GetItemID))))