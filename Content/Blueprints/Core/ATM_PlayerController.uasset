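; Player controller that sets up the main HUD, Enhanced Input mapping and game-only input, and detects interactable objects in view.
; A looping timer set at startup appears to drive a camera-forward line trace, which is skipped while the pawn is falling.
; Hit components tagged "Interactable" set the focused actor and get highlighted through custom depth, which is cleared when focus is lost.
; A load-from-slot branch is present but never runs.
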(event Custom|TraceForInteraction
  (bind _returnvalue (Game|GetPlayerCameraManager 0))
  (bind _returnvalue_2 (Transformation|GetActorLocation _returnvalue))
  (|ShouldTrace_2
    (:DontTrace
      (Variables|Default|SetFocusedObject 0)
      (bind _activecomponent (Variables|Default|GetActiveComponent)
        (:then
          (Rendering|SetRenderCustomDepth _activecomponent false))
        (:else)))
    (:Trace
      (bind (_outhit _returnvalue_3) (Collision|LineTraceByChannel _returnvalue_2 (+ _returnvalue_2 (* (Transformation|GetActorForwardVector _returnvalue) (Variables|Default|GetTraceDistance))) "TraceTypeQuery1" false (Utilities|Array|MakeArray (Game|Player|GetPlayerPawn 0)) "None"))
      (if _returnvalue_3
        (if (Components|ComponentHasTag (.HitComponent (Collision|BreakHitResult _outhit)) "Interactable")
          (Variables|Default|SetFocusedObject (.HitActor (Collision|BreakHitResult _outhit)))
          (bind _activecomponent_2 (Variables|Default|GetActiveComponent)
            (:then
              (Rendering|SetRenderCustomDepth _activecomponent_2 false))
            (:else
              _))
          (bind _output_get (Variables|Default|SetActiveComponent (.HitComponent (Collision|BreakHitResult _outhit))))
          (Rendering|SetRenderCustomDepth _output_get true)
          (else
            (Variables|Default|SetFocusedObject 0 :!label _label)
            (bind _activecomponent_3 (Variables|Default|GetActiveComponent)
              (:then
                (Rendering|SetRenderCustomDepth _activecomponent_3 false))
              (:else))))
        (else
          (goto _label))))))

(event EventBeginPlay
  (bind _returnvalue (PlayerController|LocalPlayerSubsystems|GetEnhancedInputLocalPlayerSubsystem))
  ;[0.849 0.4156 0.2145 0.5] Set Player Character Instance
  (bind _returnvalue_2 (UserInterface|CreateWidget "/Game/UI/WBP_MainHUD.WBP_MainHUD_C"))
  (UserInterface|Viewport|AddtoViewport _returnvalue_2 0)
  (bind _output_get (Variables|Default|SetGamePawn (Game|Player|GetPlayerPawn 0)))
  (bind _asbp_first_person_character (Utilities|Casting|CastToBP_FirstPersonCharacter _output_get))
  (Variables|Default|SetPlayerCharacterMesh (Variables|/Script/Engine.Character|GetMesh _asbp_first_person_character))
  (Utilities|IsValid _returnvalue
    (:Is%20Valid
      (Input|AddMappingContext _returnvalue "/Game/Blueprints/Core/Input/IMC_Player.IMC_Player" 0 "(bIgnoreAllPressedKeysUntilRelease=True,bForceImmediately=False,bNotifyUserSettings=False)")
      (Input|SetInputModeGameOnly self false)
      (Utilities|Time|SetTimerbyEvent (EventDispatchers|CreateEvent :!event Custom|TraceForInteraction) 0.05 true))))

(fn ConstructionScript)